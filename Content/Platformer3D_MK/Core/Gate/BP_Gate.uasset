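; BP_Gate is a forcefield gate that opens for a main character carrying the matching keys.
; On BeginPlay it creates a dynamic material for the forcefield mesh and tints it with the gate's color.
; When BP_MainCharacter enters the interaction zone, its KeysCollected tags are checked against the GateType query, playing a lever or locked sound.
; A match disables forcefield collision and runs a timeline that animates the material's opacity.
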(event `self.ReceiveBeginPlay`
  (bind _returnvalue (`PrimitiveComponent.CreateDynamicMaterialInstance` (`self.SM_Forcefield`) 0 "/Game/TeachersMarketplace/Assets/Architecture/Gate/Material/MI_forcefield.MI_forcefield" "None"))
  (set `self.ForceFieldDynMatRef` _returnvalue)
  (`MaterialInstanceDynamic.SetVectorParameterValue` (`self.ForceFieldDynMatRef`) "ColorMultiplier" (`self.GateForceFieldColor`)))

(event `self.GateInteractionZone.OnComponentBeginOverlap`
  (params (OverlappedComponent :type "PrimitiveComponent Object Reference") (OtherActor :type "Actor Object Reference") (OtherComp :type "PrimitiveComponent Object Reference") (OtherBodyIndex :type Integer) (bFromSweep :type Boolean) (SweepResult :type "HitResult Structure (by ref)"))
  (bind _asbp_main_character (cast `/Game/Platformer3D_MK/Core/Player/BP_MainCharacter` OtherActor))
  (if (`BlueprintGameplayTagLibrary.DoesContainerMatchTagQuery` (`/Game/Platformer3D_MK/Core/Player/BP_MainCharacter.KeysCollected` _asbp_main_character) (`self.GateType`))
    (`self.OpenGate`)
    (`GameplayStatics.PlaySound2D` "/Game/Hour_of_Code/Audio/SFX_lever.SFX_lever" 1.0 1.0 0.0 null null)
    (else
      (`GameplayStatics.PlaySound2D` "/Game/Hour_of_Code/Audio/SFX_door_locked.SFX_door_locked" 1.0 1.0 0.0 null null))))

(event `OpenGate`
  (`PrimitiveComponent.SetCollisionEnabled` (`self.SM_Forcefield`) "NoCollision")
  (bind (_direction _opacity) (`Timeline|T_OpeningGate`)
    (:`Update`
      (`MaterialInstanceDynamic.SetScalarParameterValue` (`self.ForceFieldDynMatRef`) "Opacity" _opacity))))

(fn `UserConstructionScript`)