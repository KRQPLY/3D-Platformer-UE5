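; BP_HeightRespawn is a trigger volume, likely for falls, that costs the player health and respawns them.
; On box overlap it calls LowerHealthPoints on the player character, without checking which actor entered.
; A non-negative result teleports the overlapping actor to the game mode's RespawnPoint.
; Otherwise it stores the current level name in the game instance for restart and loads LoseScreen as a level instance.
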(event `self.Box.OnComponentBeginOverlap`
  (params (OverlappedComponent :type "PrimitiveComponent Object Reference") (OtherActor :type "Actor Object Reference") (OtherComp :type "PrimitiveComponent Object Reference") (OtherBodyIndex :type Integer) (bFromSweep :type Boolean) (SweepResult :type "HitResult Structure (by ref)"))
  (bind _asbp_main_character (cast `/Game/Platformer3D_MK/Core/Player/BP_MainCharacter` (`GameplayStatics.GetPlayerCharacter` 0)))
  (bind _healthpoints (`/Game/Platformer3D_MK/Core/Player/BP_MainCharacter.LowerHealthPoints` _asbp_main_character))
  (if (>= _healthpoints 0)
    (bind _asgm_platformer_3d_mk (cast `/Game/Platformer3D_MK/Core/Framework/GM_Platformer3D_MK` (`GameplayStatics.GetGameMode`)))
    (bind (_respawnpoint_location _respawnpoint_rotation) (`KismetMathLibrary.BreakTransform` (`/Game/Platformer3D_MK/Core/Framework/GM_Platformer3D_MK.RespawnPoint` _asgm_platformer_3d_mk)))
    (`self.K2_TeleportTo` OtherActor _respawnpoint_location _respawnpoint_rotation)
    (else
      (bind _asmain_game_instance (cast `/Game/Platformer3D_MK/Instance/MainGameInstance` (`GameplayStatics.GetGameInstance`)))
      (bind _returnvalue (`GameplayStatics.GetCurrentLevelName` true))
      (set `/Game/Platformer3D_MK/Instance/MainGameInstance.LevelToRestartName` (`KismetStringLibrary.Conv_StringToName` _returnvalue) _asmain_game_instance)
      (`LevelStreamingDynamic.LoadLevelInstance` "LoseScreen" (0.0 0.0 0.0) (struct) "" null))))

(fn `UserConstructionScript`)