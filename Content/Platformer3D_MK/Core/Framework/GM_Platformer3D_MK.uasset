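; Game mode for the 3D platformer that owns the HUD, the player's respawn point and the level-win transition.
; On BeginPlay it creates the HUD, shows default health and takes the PlayerStart transform as the initial respawn point.
; Helper functions update health text, add blue or red key icons, and move the respawn point while resetting the previous checkpoint.
; WinTheGame triggers the character's celebration, then opens the next level after a short delay.
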(event `self.ReceiveBeginPlay`
  (bind _returnvalue (`|CreateWidget` "/Game/Platformer3D_MK/Core/HUD/W_GameHUD.W_GameHUD_C"))
  (bind _output_get (set `self.GameHUD` _returnvalue))
  (`self.UpdateHUDHealth` (`self.DefaultHealthPoints`))
  (`UserWidget.AddToViewport` _output_get 0)
  (bind _returnvalue_2 (`GameplayStatics.GetActorOfClass` "/Script/Engine.PlayerStart"))
  (set `self.RespawnPoint` (`self.GetTransform` _returnvalue_2)))

(event `WinTheGame`
  (params (NextLevel :type String))
  (bind _asbp_main_character (cast `/Game/Platformer3D_MK/Core/Player/BP_MainCharacter` (`GameplayStatics.GetPlayerCharacter` 0)))
  (`/Game/Platformer3D_MK/Core/Player/BP_MainCharacter.EnterCelebration` _asbp_main_character)
  (`KismetSystemLibrary.Delay` 3.0)
  (`GameplayStatics.OpenLevel` (`KismetStringLibrary.Conv_StringToName` NextLevel)))

(fn `UpdateHUDHealth`
  (params (HealthPoints :type Integer))
  (if (>= HealthPoints 0)
    (bind _asw_game_hud (cast `/Game/Platformer3D_MK/Core/HUD/W_GameHUD` (`self.GameHUD`)))
    (`TextBlock.SetText` (`/Game/Platformer3D_MK/Core/HUD/W_GameHUD.HealthPoints` _asw_game_hud) (`KismetTextLibrary.Conv_IntToText` HealthPoints))))

(fn `UpdateHUDKeys`
  (params (KeyType :type String))
  (if (`KismetStringLibrary.EqualEqual_StrStr` KeyType "Key.Blue")
    (bind _asw_game_hud (cast `/Game/Platformer3D_MK/Core/HUD/W_GameHUD` (`self.GameHUD`)))
    (bind _returnvalue (`|CreateWidget` "/Game/Platformer3D_MK/Core/HUD/W_KeyBlue.W_KeyBlue_C"))
    (`HorizontalBox.AddChildToHorizontalBox` (`/Game/Platformer3D_MK/Core/HUD/W_GameHUD.KeysContainer` _asw_game_hud) _returnvalue)
    (elif (`KismetStringLibrary.EqualEqual_StrStr` KeyType "Key.Red")
      (bind _asw_game_hud_2 (cast `/Game/Platformer3D_MK/Core/HUD/W_GameHUD` (`self.GameHUD`)))
      (bind _returnvalue_2 (`|CreateWidget` "/Game/Platformer3D_MK/Core/HUD/W_KeyRed.W_KeyRed_C"))
      (`HorizontalBox.AddChildToHorizontalBox` (`/Game/Platformer3D_MK/Core/HUD/W_GameHUD.KeysContainer` _asw_game_hud_2) _returnvalue_2))))

(fn `UpdateRespawnPoint`
  (params (RespawnPoint :type "Transform Structure") (CheckpointRef :type "/Game/Platformer3D_MK/Core/RespawnSystem/BP_Checkpoint Object Reference"))
  (bind _currentcheckpoint_ref (`self.CurrentCheckpoint Ref`))
  (`|ExecutionSequence`
    (:`then_0`
      (if (`KismetSystemLibrary.IsValid` _currentcheckpoint_ref)
        (`/Game/Platformer3D_MK/Core/RespawnSystem/BP_Checkpoint.ReturnToNormal` _currentcheckpoint_ref)))
    (:`then_1`
      (set `self.RespawnPoint` RespawnPoint)
      (set `self.CurrentCheckpoint Ref` CheckpointRef))))

(fn `UserConstructionScript`)